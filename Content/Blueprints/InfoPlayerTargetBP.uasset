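; Player Blueprint for placing objects in the world, with an on-screen widget for the selected item.
; A per-frame camera line trace stores the impact point and normal, and right mouse spawns the selected class there, oriented to the surface.
; Q cycles through the object list with wraparound, then updates the cube, cylinder and cone highlight colors, which all test for index zero.
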(event Custom|ChangeItem
  (if (>= (Variables|Default|GetCurrentItem) 0)
    (Variables|Default|SetCurrentItem (+ (Variables|Default|GetCurrentItem) 1))
    (Variables|Default|SetObjects (Utilities|Array|Get(acopy) (Variables|Default|GetListOfObjects) (Variables|Default|GetCurrentItem)))
    (if (== (Variables|Default|GetCurrentItem) (Variables|Default|GetTotalObjects))
      (Variables|Default|SetCurrentItem (- (Variables|Default|GetCurrentItem) (Variables|Default|GetTotalObjects)))
      (Variables|Default|SetObjects (Utilities|Array|Get(acopy) (Variables|Default|GetListOfObjects) (Variables|Default|GetCurrentItem))))))

(event Custom|ChangeUIItem
  (Utilities|FlowControl|Sequence
    (:then_0
      (if (== (Variables|Default|GetCurrentItem) 0)
        (Variables|Default|SetCubeOpacity "(R=1.000000,G=1.000000,B=1.000000,A=1.000000)")
        (else
          (Variables|Default|SetCubeOpacity "(R=0.161458,G=0.161458,B=0.161458,A=1.000000)"))))
    (:then_1
      (if (== (Variables|Default|GetCurrentItem) 0)
        (Variables|Default|SetCylinderOpacity "(R=1.000000,G=1.000000,B=1.000000,A=1.000000)")
        (else
          (Variables|Default|SetCylinderOpacity "(R=0.286458,G=0.280490,B=0.280490,A=1.000000)"))))
    (:then_2
      (if (== (Variables|Default|GetCurrentItem) 0)
        (Variables|Default|SetConeOpacity "(R=1.000000,G=1.000000,B=1.000000,A=1.000000)")
        (else
          (Variables|Default|SetConeOpacity "(R=0.192708,G=0.192708,B=0.192708,A=1.000000)"))))))

(event EventTick
  (params (DeltaSeconds :type Float%20%28single-precision%29))
  (bind _followcamera (Variables|Default|GetFollowCamera))
  (bind _returnvalue (Transformation|GetWorldLocation _followcamera))
  (bind _outhit (Collision|LineTraceForObjects _returnvalue (+ (* (Math|Vector|GetForwardVector _followcamera) 1e+03) _returnvalue) (Utilities|Array|MakeArray "ObjectTypeQuery1" "ObjectTypeQuery2") false 0 "ForOneFrame"))
  (if true
    (Variables|Default|SetImpactLocation (.Location (Collision|BreakHitResult _outhit)))
    (Variables|Default|SetNormal (.Normal (Collision|BreakHitResult _outhit)))
    (Variables|Default|SetHitActor (.HitActor (Collision|BreakHitResult _outhit)))))

(event EventBeginPlay
  (Variables|Default|SetTotalObjects (Utilities|Array|Length (Variables|Default|GetListOfObjects)))
  (bind _returnvalue (UserInterface|CreateWidget "/Game/Blueprints/UI_ChangeItem.UI_ChangeItem_C"))
  (UserInterface|Viewport|AddtoViewport _returnvalue 0))

(event Input|MouseEvents|RightMouseButton
  (params (Key :type Key%20Structure))
  (:Pressed
    (Game|SpawnActorfromClass (Variables|Default|GetObjects) (Math|Transform|MakeTransform (Variables|Default|GetImpactLocation) (Math|Rotator|MakeRotfromZ (Variables|Default|GetNormal))) "Undefined" 0 0)))

(event Input|KeyboardEvents|Q
  (params (Key :type Key%20Structure))
  (:Pressed
    (Utilities|FlowControl|Sequence
      (:then_0
        (CallFunction|ChangeItem))
      (:then_1
        (CallFunction|ChangeUIItem)))))

(fn ConstructionScript)